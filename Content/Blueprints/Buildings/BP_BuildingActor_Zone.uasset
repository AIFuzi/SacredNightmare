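; BP_BuildingActor_Zone is a building actor with a spherical zone that tracks and notifies actors that overlap it.
; The construction script sizes the sphere from ZoneRadius.
; Begin overlap calls ZoneOverlapStart, which adds the actor to OverlappedActors and sends it a zone-start message.
; ZoneOverlapEnd removes the actor and sends a stop message, but the event graph never calls it.
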(event `self.Sphere.OnComponentBeginOverlap`
  (params (OverlappedComponent :type "PrimitiveComponent Object Reference") (OtherActor :type "Actor Object Reference") (OtherComp :type "PrimitiveComponent Object Reference") (OtherBodyIndex :type Integer) (bFromSweep :type Boolean) (SweepResult :type "HitResult Structure (by ref)"))
  (`self.ZoneOverlapStart` OtherActor))

(fn `UserConstructionScript`
  (`SphereComponent.SetSphereRadius` (`self.Sphere`) (`self.ZoneRadius`) true))

(fn `ZoneOverlapEnd`
  (params (Actor :type "Actor Object Reference"))
  (`KismetArrayLibrary.Array_RemoveItem` (`self.OverlappedActors`) Actor)
  (message `/Game/Blueprints/Data/BI_BuildingZone.OverlapBuildingZoneStop` Actor))

(fn `ZoneOverlapStart`
  (params (Actor :type "Actor Object Reference"))
  (`KismetArrayLibrary.Array_AddUnique` (`self.OverlappedActors`) Actor)
  (message `/Game/Blueprints/Data/BI_BuildingZone.OverlapBuildingZoneStart` Actor))
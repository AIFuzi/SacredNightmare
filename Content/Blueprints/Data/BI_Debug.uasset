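; BI_Debug is a Blueprint debug helper with a PrintMessage function for showing on-screen messages.
; It prepends the caller's prefix and a colon when one is given, using the supplied color and duration.
; When the error flag is set, it replaces the prefix with an ERROR label and forces red text.
; Output goes to the screen only, not the log.
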(fn `PrintMessage`
  (params (WorldObject :type "Object Object Reference") (IsError :type Boolean) (Prefix :type String) (Message :type String) (Color :type "LinearColor Structure" :default (struct :`R` 1.0 :`G` 1.0 :`B` 1.0 :`A` 1.0)) (Duration :type "Float (double-precision)"))
  (locals (L_Message :type String) (L_Prefix :type String) (L_IsError :type Boolean) (L_Color :type "LinearColor Structure" :default (struct :`R` 1.0 :`G` 1.0 :`B` 1.0)) (L_Duration :type "Float (double-precision)"))
  (bind _l_message (`local.L_Message`))
  (bind _returnvalue (not (`local.L_IsError`)))
  (set `local.L_IsError` IsError)
  (set `local.L_Prefix` Prefix)
  (set `local.L_Message` Message)
  (set `local.L_Color` Color)
  (set `local.L_Duration` Duration)
  (`KismetSystemLibrary.PrintString` WorldObject (`KismetMathLibrary.SelectString` (`KismetMathLibrary.SelectString` (`KismetStringLibrary.Concat_StrStr` (`local.L_Prefix`) ": " (`local.L_Message`)) _l_message (> (`KismetStringLibrary.Len` (`local.L_Prefix`)) 0)) (`KismetStringLibrary.Concat_StrStr` "ERROR: " _l_message) _returnvalue) true false (`KismetMathLibrary.SelectColor` (`local.L_Color`) (struct :`R` 1.0 :`A` 1.0) _returnvalue) (`local.L_Duration`)))
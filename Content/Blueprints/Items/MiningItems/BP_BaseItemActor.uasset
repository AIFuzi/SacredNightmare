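; Base actor for a mineable item that goes into the interacting player's or owner's inventory once mined enough.
; Interact, when not on cooldown, updates the condition and, once it reaches the item struct's MiningCondition, adds the item through the owner's BPInventoryComponent and returns true.
; Tick prints the current condition as a debug message; the OnItemMining binding is unconnected.
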(event `self.ReceiveBeginPlay`)

(event `OnItemMining_Event_0`)

(event `self.ReceiveTick`
  (params (DeltaSeconds :type "Float (single-precision)"))
  (`/Game/Blueprints/Data/BI_Debug.PrintMessage` self false "Current condition" (`KismetStringLibrary.Conv_IntToString` (`self.GetCurrentCondition`)) (struct :`G` 0.08531 :`B` 1.0 :`A` 1.0)))

(fn `Interact`
  (params (InteractOwner :type "/Game/Blueprints/Characters/Player/BP_Player Object Reference"))
  (returns (Succeess :type Boolean))
  (bind (_itemstruct_itemname _itemstruct_miningcondition) (break `ItemStruct` (`self.ItemStruct`)))
  (if (not (`self.GetIsCooldown`))
    (`self.UpdateCondition`)
    (if (>= (`self.GetCurrentCondition`) _itemstruct_miningcondition)
      (`InventoryComponent.AddItemToInventory` (`/Game/Blueprints/Characters/Player/BP_Player.BP_InventoryComponent` InteractOwner) (`self.ItemStruct`))
      (return true))))

(fn `UserConstructionScript`)
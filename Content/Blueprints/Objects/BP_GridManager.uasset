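; BP_GridManager is a grid manager actor that holds cell actors and finds the position of the one nearest a given point.
; BeginPlay calls CreateGridWorld, whose body is not shown, while PupulateGrid sits unwired.
; PupulateGrid spawns a square of BP_GridCell actors into GridArray, multiplying coordinates by the half-grid offset rather than subtracting it.
; GetClossetGridPositiond linearly scans GridArray by distance to return the closest cell location.
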(event `self.ReceiveBeginPlay`
  (`self.CreateGridWorld`))

(fn `GetClossetGridPositiond`
  (params (Position :type "Vector Structure"))
  (returns (Return :type "Vector Structure"))
  (locals (CloseetPosition :type "Vector Structure") (ClossetDistance :type "Float (double-precision)") (L_Position :type "Vector Structure"))
  (bind _returnvalue (`self.K2_GetActorLocation` (`|GetArrayItem` (`self.GridArray`))))
  (bind _output_get (set `local.L_Position` Position))
  (set `local.CloseetPosition` _returnvalue)
  (set `local.ClossetDistance` (`KismetMathLibrary.Vector_Distance` _output_get _returnvalue))
  (for _array_element (`self.GridArray`)
    (bind _returnvalue_2 (`self.K2_GetActorLocation` _array_element))
    (bind _returnvalue_3 (`KismetMathLibrary.Vector_Distance` _returnvalue_2 (`local.L_Position`)))
    (if (< _returnvalue_3 (`local.ClossetDistance`))
      (set `local.CloseetPosition` _returnvalue_2)
      (set `local.ClossetDistance` _returnvalue_3)))
  (return (`local.CloseetPosition`)))

(fn `PupulateGrid`
  (locals (WorldOffset :type "Float (double-precision)"))
  (bind (_returnvalue_x _returnvalue_y _returnvalue_z) (`KismetMathLibrary.BreakVector` (`self.K2_GetActorLocation`)))
  (bind _worldgridsize (`self.WorldGridSize`))
  (bind _worldgridsize_2 (`self.WorldGridSize`))
  (bind _returnvalue (`KismetMathLibrary.FTrunc` (`local.WorldOffset`)))
  (`KismetArrayLibrary.Array_Clear` (`self.GridArray`))
  (set `local.WorldOffset` (- (* (* (`self.GridSize`) _worldgridsize_2) 0.5) (* _worldgridsize_2 0.5)))
  (for _index (range (`self.GridSize`))
    (for _index_2 (range (`self.GridSize`))
      (bind _returnvalue_2 (`|SpawnActorFromClass` "/Game/Blueprints/Objects/BP_GridCell.BP_GridCell_C" (`KismetMathLibrary.MakeTransform` (`KismetMathLibrary.MakeVector` (`KismetMathLibrary.Conv_IntToDouble` (* (* _index_2 _worldgridsize) _returnvalue)) (`KismetMathLibrary.Conv_IntToDouble` (* (* _worldgridsize _index) _returnvalue)) (- _returnvalue_z (/ _returnvalue_z 2.0)))) "AlwaysSpawn" "OverrideRootScale" null null))
      (`KismetArrayLibrary.Array_Add` (`self.GridArray`) _returnvalue_2))))

(fn `UserConstructionScript`)